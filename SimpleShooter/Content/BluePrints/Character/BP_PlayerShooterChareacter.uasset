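; Player shooter character Blueprint that adds weapon pickup animation and cover component setup on top of its parent class.
; GrabbingtheWeapon either plays a right-hand pickup montage with movement locked for its duration, or a generic item pickup montage.
; The construction script starts a looping, near per-frame timer calling BPCoverComponent's "ContructionScript" function by name, unless already active.
; Cover-entry animation and intro sound fragments are disconnected.
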(event `self.ReceiveBeginPlay`
  (`parent.ReceiveBeginPlay`))

(event `self.ReceiveTick`
  (params (DeltaSeconds :type "Float (single-precision)"))
  (`parent.ReceiveTick` DeltaSeconds))

(event `InputAction|Crouch`
  (params (Key :type "Key Structure")))

(event `self.GrabbingTheWeapon`
  (if (`self.bWantsToGrabWeapon`)
    (`CharacterMovementComponent.DisableMovement` (`self.CharacterMovement`))
    (bind _returnvalue (`self.PlayAnimMontage` "/Game/Animation/Movement_Animset/RootMotion/PickUp_RH_Montage.PickUp_RH_Montage"))
    (`KismetSystemLibrary.Delay` _returnvalue)
    (`CharacterMovementComponent.SetMovementMode` (`self.CharacterMovement`) "MOVE_Walking" 0)
    (else
      (`self.PlayAnimMontage` "/Game/Pick_Up_Item__1__Anim_Montage.Pick_Up_Item__1__Anim_Montage" 0.8))))

(fn `UserConstructionScript`
  (if (not (`KismetSystemLibrary.K2_IsTimerActiveHandle` (`self.Construction Timer Handle`)))
    (bind _returnvalue (`KismetSystemLibrary.K2_SetTimer` (`self.BP_CoverComponent`) "ContructionScript" 0.0016 true))
    (set `self.Construction Timer Handle` _returnvalue)
    (`parent.UserConstructionScript`)))