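; Animation modifier that auto-generates RightFoot and LeftFoot sync markers on an animation sequence, on a FootSyncNotify track.
; For each foot, it composes bone poses up to but excluding root on every frame to get the foot's root-relative position.
; The Y value is keyed into SyncCurve, shared by both feet.
; A DoOnce reset while Y is positive limits markers to crossings to zero or below, skipping frame 0.
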(event `self.OnApply`
  (params (AnimationSequence :type "AnimSequence Object Reference"))
  (set `self.Animation Sequence` AnimationSequence)
  (`AnimationBlueprintLibrary.AddCurve` (`self.Animation Sequence`) "SyncCurve")
  (`AnimationBlueprintLibrary.AddAnimationNotifyTrack` (`self.Animation Sequence`) "FootSyncNotify")
  (for _index (range (+ (`AnimationBlueprintLibrary.GetNumFrames` (`self.Animation Sequence`)) 1))
    (set `self.Index` _index)
    (set `self.Transform` (`KismetMathLibrary.MakeTransform` (0.0 0.0 0.0)))
    (for _array_element (`AnimationBlueprintLibrary.FindBonePathToRoot` (`self.Animation Sequence`) "Foot_R")
      (if (== _array_element "root")
        (break)
        (else
          (set `self.Transform` (`KismetMathLibrary.ComposeTransforms` (`self.Transform`) (`AnimationBlueprintLibrary.GetBonePoseForFrame` (`self.Animation Sequence`) _array_element (`self.Index`)))))))
    (`AnimationBlueprintLibrary.AddFloatCurveKey` (`self.Animation Sequence`) "SyncCurve" (`AnimationBlueprintLibrary.GetTimeAtFrame` (`self.Animation Sequence`) (`self.Index`)) (.y (.location (`self.Transform`))))
    (if (> (.y (.location (`self.Transform`))) 0.0)
      (goto _label :!via `Reset`)
      (else
        (`/Engine/EditorBlueprintResources/StandardMacros.DoOnce` false :!label _label
          (:`Completed`
            (if (not (== (`self.Index`) 0))
              (`AnimationBlueprintLibrary.AddAnimationSyncMarker` (`self.Animation Sequence`) "RightFoot" (`AnimationBlueprintLibrary.GetTimeAtFrame` (`self.Animation Sequence`) (`self.Index`)) "FootSyncNotify")))))))
  (for _index_2 (range (+ (`AnimationBlueprintLibrary.GetNumFrames` (`self.Animation Sequence`)) 1))
    (set `self.Index` _index_2)
    (set `self.Transform` (`KismetMathLibrary.MakeTransform` (0.0 0.0 0.0)))
    (for _array_element_2 (`AnimationBlueprintLibrary.FindBonePathToRoot` (`self.Animation Sequence`) "Foot_L")
      (if (== _array_element_2 "root")
        (break)
        (else
          (set `self.Transform` (`KismetMathLibrary.ComposeTransforms` (`self.Transform`) (`AnimationBlueprintLibrary.GetBonePoseForFrame` (`self.Animation Sequence`) _array_element_2 (`self.Index`)))))))
    (`AnimationBlueprintLibrary.AddFloatCurveKey` (`self.Animation Sequence`) "SyncCurve" (`AnimationBlueprintLibrary.GetTimeAtFrame` (`self.Animation Sequence`) (`self.Index`)) (.y (.location (`self.Transform`))))
    (if (> (.y (.location (`self.Transform`))) 0.0)
      (goto _label_2 :!via `Reset`)
      (else
        (`/Engine/EditorBlueprintResources/StandardMacros.DoOnce` false :!label _label_2
          (:`Completed`
            (if (not (== (`self.Index`) 0))
              (`AnimationBlueprintLibrary.AddAnimationSyncMarker` (`self.Animation Sequence`) "LeftFoot" (`AnimationBlueprintLibrary.GetTimeAtFrame` (`self.Animation Sequence`) (`self.Index`)) "FootSyncNotify"))))))))