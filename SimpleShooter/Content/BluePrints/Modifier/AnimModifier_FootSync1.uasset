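; Animation Modifier that auto-places RightFoot and LeftFoot sync markers on a FootSyncNotify track of an animation sequence.
; Each frame, FindWorldLocation composes bone poses from Foot_R and Foot_L up to, excluding, root.
; When the lower foot's Y changes sign, a DoOnce-gated marker lands on whichever frame is nearer zero.
; AcceptableThreshold limits that nearest distance, but the right-foot check negates the distance before comparing.
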(event `self.OnApply`
  (params (AnimationSequence :type "AnimSequence Object Reference"))
  (bind _returnvalue (`KismetMathLibrary.MakeTransform` (0.0 0.0 0.0)))
  (bind _index (`self.Index`))
  (bind _transforml (`self.TransformL`))
  (bind _index_2 (`self.Index`))
  (bind _transformr (`self.TransformR`))
  (bind _prevtransformr (`self.PrevTransformR`))
  (bind _prevtransforml (`self.PrevTransformL`))
  (bind _returnvalue_2 (`KismetMathLibrary.Abs` (.y (.location _transforml))))
  (bind _returnvalue_3 (`KismetMathLibrary.Abs` (.y (.location _transformr))))
  (bind _returnvalue_4 (`KismetMathLibrary.Abs` (.y (.location _prevtransforml))))
  (bind _returnvalue_5 (`KismetMathLibrary.Abs` (.y (.location _prevtransformr))))
  (bind _returnvalue_6 (< _returnvalue_2 _returnvalue_4))
  (bind _returnvalue_7 (< _returnvalue_3 _returnvalue_5))
  (set `self.Animation Sequence` AnimationSequence)
  (`AnimationBlueprintLibrary.AddAnimationNotifyTrack` (`self.Animation Sequence`) "FootSyncNotify")
  (for _index_3 (range (+ (`AnimationBlueprintLibrary.GetNumFrames` (`self.Animation Sequence`)) 1))
    (set `self.Index` _index_3)
    (set `self.PrevTransformR` (`self.TransformR`))
    (set `self.PrevTransformL` (`self.TransformL`))
    (set `self.TransformR` _returnvalue)
    (set `self.TransformL` _returnvalue)
    (bind _worldtransform (`self.FindWorldLocation` "Foot_R" (`self.Index`) (`self.Animation Sequence`)))
    (set `self.TransformR` _worldtransform)
    (bind _worldtransform_2 (`self.FindWorldLocation` "Foot_L" (`self.Index`) (`self.Animation Sequence`)))
    (set `self.TransformL` _worldtransform_2)
    (`|ExecutionSequence`
      (:`then_0`
        (set `self.FlagR` _returnvalue_7)
        (if (and (< (* (`KismetMathLibrary.SelectFloat` _returnvalue_3 _returnvalue_5 _returnvalue_7) -1.0) (`self.AcceptableThreshold`)) (< (* (.y (.location _transformr)) (.y (.location _prevtransformr))) 0.0))
          (if (< (.z (.location (`self.TransformR`))) (.z (.location (`self.TransformL`))))
            (if (!= (`self.Index`) 0)
              (`/Engine/EditorBlueprintResources/StandardMacros.DoOnce` false :!label _label
                (:`Completed`
                  (`AnimationBlueprintLibrary.AddAnimationSyncMarker` (`self.Animation Sequence`) "RightFoot" (`AnimationBlueprintLibrary.GetTimeAtFrame` (`self.Animation Sequence`) (`KismetMathLibrary.SelectInt` _index (- _index 1) (`self.FlagR`))) "FootSyncNotify")))))
          (else
            (goto _label :!via `Reset`))))
      (:`then_1`
        (set `self.FlagL` _returnvalue_6)
        (if (and (< (`KismetMathLibrary.SelectFloat` _returnvalue_2 _returnvalue_4 _returnvalue_6) (`self.AcceptableThreshold`)) (< (* (.y (.location _transforml)) (.y (.location _prevtransforml))) 0.0))
          (if (< (.z (.location (`self.TransformL`))) (.z (.location (`self.TransformR`))))
            (if (!= (`self.Index`) 0)
              (`/Engine/EditorBlueprintResources/StandardMacros.DoOnce` false :!label _label_2
                (:`Completed`
                  (`AnimationBlueprintLibrary.AddAnimationSyncMarker` (`self.Animation Sequence`) "LeftFoot" (`AnimationBlueprintLibrary.GetTimeAtFrame` (`self.Animation Sequence`) (`KismetMathLibrary.SelectInt` _index_2 (- _index_2 1) (`self.FlagL`))) "FootSyncNotify")))))
          (else
            (goto _label_2 :!via `Reset`)))))))

(fn `FindWorldLocation`
  (params (BoneName :type Name) (Index :type Integer) (AnimSeq :type "AnimSequence Object Reference"))
  (returns (WorldTransform :type "Transform Structure"))
  (locals (Transform :type "Transform Structure"))
  (set `local.Transform` (`KismetMathLibrary.MakeTransform` (0.0 0.0 0.0)))
  (for _array_element (`AnimationBlueprintLibrary.FindBonePathToRoot` AnimSeq BoneName)
    (if (== _array_element "root")
      (break)
      (else
        (set `local.Transform` (`KismetMathLibrary.ComposeTransforms` (`local.Transform`) (`AnimationBlueprintLibrary.GetBonePoseForFrame` AnimSeq _array_element Index))))))
  (return (`local.Transform`)))